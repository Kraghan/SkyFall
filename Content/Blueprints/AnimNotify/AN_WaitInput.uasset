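; Anim notify state that opens an input window for light and/or heavy attack requests on the ALS AnimMan character during an animation.
; Begin ORs its two wait flags into the character's allowed attack requests.
; End calls ProcessInputRequest, then XORs the flags with the current permissions to withdraw what it granted.
; Both events print debug text, and the notify name reflects which inputs it waits for.
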(fn `GetNotifyName`
  (returns (ReturnValue :type String))
  (bind _bwaitheavyattack (`self.bWaitHeavyAttack`))
  (if (`self.bWaitLightAttack`)
    (if _bwaitheavyattack
      (return "Wait both input")
      (else
        (return "Wait light input")))
    (elif _bwaitheavyattack
      (return "Wait heavy input")
      (else
        (return "Wait none")))))

(fn `Received_NotifyBegin`
  (params (MeshComp :type "SkeletalMeshComponent Object Reference") (Animation :type "AnimSequenceBase Object Reference") (TotalDuration :type "Float (double-precision)"))
  (returns (ReturnValue :type Boolean))
  (bind _asals_anim_man_character_bp (cast `/Game/AdvancedLocomotionV4/Blueprints/CharacterLogic/ALS_AnimMan_CharacterBP` (`ActorComponent.GetOwner` MeshComp)))
  (`/Game/AdvancedLocomotionV4/Blueprints/CharacterLogic/ALS_AnimMan_CharacterBP.AllowRequestAttack` _asals_anim_man_character_bp (or (`self.bWaitLightAttack`) (`/Game/AdvancedLocomotionV4/Blueprints/CharacterLogic/ALS_AnimMan_CharacterBP.bCanRequestLightAttack` _asals_anim_man_character_bp)) (or (`self.bWaitHeavyAttack`) (`/Game/AdvancedLocomotionV4/Blueprints/CharacterLogic/ALS_AnimMan_CharacterBP.bCanRequestHeavyAttack` _asals_anim_man_character_bp)))
  (`KismetSystemLibrary.PrintString` _asals_anim_man_character_bp "Go ! ")
  (return false))

(fn `Received_NotifyEnd`
  (params (MeshComp :type "SkeletalMeshComponent Object Reference") (Animation :type "AnimSequenceBase Object Reference"))
  (returns (ReturnValue :type Boolean))
  (bind _asals_anim_man_character_bp (cast `/Game/AdvancedLocomotionV4/Blueprints/CharacterLogic/ALS_AnimMan_CharacterBP` (`ActorComponent.GetOwner` MeshComp)))
  (`/Game/AdvancedLocomotionV4/Blueprints/CharacterLogic/ALS_AnimMan_CharacterBP.ProcessInputRequest` _asals_anim_man_character_bp)
  (`/Game/AdvancedLocomotionV4/Blueprints/CharacterLogic/ALS_AnimMan_CharacterBP.AllowRequestAttack` _asals_anim_man_character_bp (xor (`self.bWaitLightAttack`) (`/Game/AdvancedLocomotionV4/Blueprints/CharacterLogic/ALS_AnimMan_CharacterBP.bCanRequestLightAttack` _asals_anim_man_character_bp)) (xor (`self.bWaitHeavyAttack`) (`/Game/AdvancedLocomotionV4/Blueprints/CharacterLogic/ALS_AnimMan_CharacterBP.bCanRequestHeavyAttack` _asals_anim_man_character_bp)))
  (`KismetSystemLibrary.PrintString` _asals_anim_man_character_bp "End" true true (struct :`R` 1.0 :`A` 1.0))
  (return false))