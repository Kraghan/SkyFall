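; Anim notify state that opens a melee damage window on the player character or boss during an animation.
; On begin, it casts the mesh owner to ALS_AnimMan_CharacterBP, falling back to BP_Boss, then enables that actor's hitbox and sets ActualDamage from its Damages variable.
; On end, it disables the hitbox, resetting ActualDamage to zero for the ALS character only.
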(fn `Received_NotifyBegin`
  (params (MeshComp :type "SkeletalMeshComponent Object Reference") (Animation :type "AnimSequenceBase Object Reference") (TotalDuration :type "Float (double-precision)"))
  (returns (ReturnValue :type Boolean))
  (bind _returnvalue (`ActorComponent.GetOwner` MeshComp))
  (bind _asals_anim_man_character_bp (cast `/Game/AdvancedLocomotionV4/Blueprints/CharacterLogic/ALS_AnimMan_CharacterBP` _returnvalue)
    (:`then`
      (`/Game/AdvancedLocomotionV4/Blueprints/CharacterLogic/ALS_AnimMan_CharacterBP.SetHitBoxActivation` _asals_anim_man_character_bp true)
      (set `/Game/AdvancedLocomotionV4/Blueprints/CharacterLogic/ALS_AnimMan_CharacterBP.ActualDamage` (`self.Damages`) _asals_anim_man_character_bp)
      (return false))
    (:`CastFailed`
      (bind _asbp_boss (cast `/Game/Blueprints/Character/BP_Boss` _returnvalue))
      (`/Game/Blueprints/Character/BP_Boss.SetHitBoxState` _asbp_boss true)
      (set `/Game/Blueprints/Character/BP_Boss.ActualDamage` (`self.Damages`) _asbp_boss))))

(fn `Received_NotifyEnd`
  (params (MeshComp :type "SkeletalMeshComponent Object Reference") (Animation :type "AnimSequenceBase Object Reference"))
  (returns (ReturnValue :type Boolean))
  (bind _returnvalue (`ActorComponent.GetOwner` MeshComp))
  (bind _asals_anim_man_character_bp (cast `/Game/AdvancedLocomotionV4/Blueprints/CharacterLogic/ALS_AnimMan_CharacterBP` _returnvalue)
    (:`then`
      (`/Game/AdvancedLocomotionV4/Blueprints/CharacterLogic/ALS_AnimMan_CharacterBP.SetHitBoxActivation` _asals_anim_man_character_bp false)
      (set `/Game/AdvancedLocomotionV4/Blueprints/CharacterLogic/ALS_AnimMan_CharacterBP.ActualDamage` 0.0 _asals_anim_man_character_bp)
      (return false))
    (:`CastFailed`
      (bind _asbp_boss (cast `/Game/Blueprints/Character/BP_Boss` _returnvalue))
      (`/Game/Blueprints/Character/BP_Boss.SetHitBoxState` _asbp_boss false))))