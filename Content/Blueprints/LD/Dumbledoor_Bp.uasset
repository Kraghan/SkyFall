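; Tag-locked double door that swings open when the player character enters its trigger box.
; On overlap it checks the ALS player controller for TagToOpen and sends a locked notification if the tag is missing.
; With the tag, it opens once, playing an attached gate sound and a timeline that rotates both doors in opposite yaw directions.
; It also binds to the controller's tag-added event, but that handler performs no action.
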(event `self.ReceiveBeginPlay`
  (bind _asals_player_controller (cast `/Game/AdvancedLocomotionV4/Blueprints/CharacterLogic/ALS_Player_Controller` (`GameplayStatics.GetPlayerController` 0)))
  (add `/Game/AdvancedLocomotionV4/Blueprints/CharacterLogic/ALS_Player_Controller.OnTagAdded` _asals_player_controller (delegate `OnTagAdded`)))

(event `OnTagAdded`
  (params (Tag :type "GameplayTag Structure"))
  (if (== Tag (`self.TagToOpen`))
    _))

(event `self.Box.OnComponentBeginOverlap`
  (params (OverlappedComponent :type "PrimitiveComponent Object Reference") (OtherActor :type "Actor Object Reference") (OtherComp :type "PrimitiveComponent Object Reference") (OtherBodyIndex :type Integer) (bFromSweep :type Boolean) (SweepResult :type "HitResult Structure (by ref)"))
  (bind _asals_anim_man_character_bp (cast `/Game/AdvancedLocomotionV4/Blueprints/CharacterLogic/ALS_AnimMan_CharacterBP` OtherActor))
  (bind _asals_player_controller (cast `/Game/AdvancedLocomotionV4/Blueprints/CharacterLogic/ALS_Player_Controller` (`Pawn.GetController` _asals_anim_man_character_bp)))
  (if (`/Game/AdvancedLocomotionV4/Blueprints/CharacterLogic/ALS_Player_Controller.HasTag` _asals_player_controller (`self.TagToOpen`))
    (if (not (`self.IsDoorOpen`))
      (set `self.IsDoorOpen` true)
      (`GameplayStatics.SpawnSoundAttached` "/Game/Sound/GateDoor.GateDoor" (`self.Door1`) "None" (0.0 0.0 0.0) (struct) "KeepRelativeOffset" false 1.0 1.0 0.0 null null)
      (bind (_direction _doorrotation) (`Timeline|Timeline_0`)
        (:`Update`
          (`SceneComponent.K2_SetRelativeRotation` (`self.Door1`) (`KismetMathLibrary.MakeRotator` 0.0 0.0 _doorrotation) false false)
          (`SceneComponent.K2_SetRelativeRotation` (`self.Door2`) (`KismetMathLibrary.MakeRotator` 0.0 0.0 (- 0.0 _doorrotation)) false false))))
    (else
      (`/Game/AdvancedLocomotionV4/Blueprints/CharacterLogic/ALS_Player_Controller.SendNotification` _asals_player_controller "The door is locked."))))

(fn `UserConstructionScript`)