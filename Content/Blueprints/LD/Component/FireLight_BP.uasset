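; Point light Blueprint that imitates flickering firelight through random movement and color shifts.
; BeginPlay stores the light's relative location as an anchor.
; Each tick eases the light toward a new random offset around that anchor, bounded by MoveStrength.
; The same Speed eases a random blend factor that mixes Color1 and Color2 in HSV space for the light color.
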(event `self.ReceiveBeginPlay`
  (set `self.InitialPos` (`SceneComponent.RelativeLocation` (`self.PointLightComponent`))))

(event `self.ReceiveTick`
  (params (DeltaSeconds :type "Float (single-precision)"))
  (bind _movestrength (`self.MoveStrength`))
  (bind _returnvalue (`KismetMathLibrary.RandomFloatInRange` (* _movestrength -1.0) _movestrength))
  (`SceneComponent.K2_SetRelativeLocation` (`self.PointLightComponent`) (`KismetMathLibrary.VInterpTo` (`SceneComponent.RelativeLocation` (`self.PointLightComponent`)) (+ (`self.InitialPos`) (`KismetMathLibrary.MakeVector` _returnvalue _returnvalue _returnvalue)) DeltaSeconds (`self.Speed`)) false false)
  (bind _output_get (set `self.ColorLerp` (`KismetMathLibrary.FClamp` (`KismetMathLibrary.FInterpTo` (`self.ColorLerp`) (`KismetMathLibrary.RandomFloatInRange` 0.0 1.0) DeltaSeconds (`self.Speed`)))))
  (`LightComponent.SetLightColor` (`self.PointLightComponent`) (`KismetMathLibrary.LinearColorLerpUsingHSV` (`self.Color1`) (`self.Color2`) _output_get) true))

(fn `UserConstructionScript`)