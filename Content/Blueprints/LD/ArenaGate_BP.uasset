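; ArenaGate_BP is an arena gate that opens once every enemy in its assigned Enemies list is dead.
; It binds to each enemy's health component death event, rechecks the list on each death, then plays metal sounds and the OpenGate timeline.
; The timeline slides the mesh by OpenOffset along a curve.
; On BeginPlay, if the player controller already has TagToAdd, the gate opens immediately without binding.
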(event `self.ReceiveBeginPlay`
  (bind _asals_player_controller (cast `/Game/AdvancedLocomotionV4/Blueprints/CharacterLogic/ALS_Player_Controller` (`GameplayStatics.GetPlayerController` 0)))
  (if (`/Game/AdvancedLocomotionV4/Blueprints/CharacterLogic/ALS_Player_Controller.HasTag` _asals_player_controller (`self.TagToAdd`))
    (bind (_direction _opencurve) (`Timeline|OpenGate` :!label _label)
      (:`Update`
        (`SceneComponent.K2_SetRelativeLocation` (`self.StaticMeshComponent0`) (+ (`self.Relative Location`) (* (`self.OpenOffset`) _opencurve)) false false)))
    (else
      (for _array_element (`self.Enemies`)
        (add `/Game/Blueprints/Gameplay/Component/Health_Component_BP.OnDie` (`/Game/AdvancedLocomotionV4/Blueprints/CharacterLogic/ALS_AnimMan_CharacterBP.Health_Component_BP` _array_element) (delegate `OnDie`)))
      (set `self.Relative Location` (`SceneComponent.RelativeLocation` (`self.StaticMeshComponent0`))))))

(event `OnDie`
  (params (DamageTakenBeforeDying :type "Float (double-precision)") (HitLocation :type "Vector Structure"))
  (set `self.AllDead` true)
  (for _array_element (`self.Enemies`)
    (`/Engine/EditorBlueprintResources/StandardMacros.IsValid` _array_element
      (:`Is Valid`
        (if (not (`/Game/Blueprints/Gameplay/Component/Health_Component_BP.IsDead` (`/Game/AdvancedLocomotionV4/Blueprints/CharacterLogic/ALS_AnimMan_CharacterBP.Health_Component_BP` _array_element)))
          (set `self.AllDead` false)))))
  (if (`self.AllDead`)
    (`GameplayStatics.PlaySoundAtLocation` "/Game/Sound/160047__jorickhoofd__metal-rattle.160047__jorickhoofd__metal-rattle" (0.0 0.0 0.0) (struct) 1.0 1.0 0.0 null null null)
    (`GameplayStatics.PlaySoundAtLocation` "/Game/Sound/530061__magnuswaker__gates-of-hell-2-gate-slam-2.530061__magnuswaker__gates-of-hell-2-gate-slam-2" (0.0 0.0 0.0) (struct) 1.0 1.0 0.5 null null null)
    (goto _label)))

(fn `UserConstructionScript`)