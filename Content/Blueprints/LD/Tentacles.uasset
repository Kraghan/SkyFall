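; Tentacles level-design actor that plays looping or ambient audio, reacts to damage and dissolves away when killed.
; On begin play its audio component starts from a random time offset, likely to desync multiple instances.
; Health component damage events spawn an attached hit-creature sound on the tentacle mesh.
; On death, after a configurable delay, a timeline drives the "Amount" parameter of a dynamic material instance, then destroys the actor.
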(event `self.ReceiveBeginPlay`
  (`AudioComponent.Play` (`self.Audio`) (`KismetMathLibrary.RandomFloatInRange` 0.0 10.0)))

(event `self.Health_Component_BP.OnDie`
  (params (DamageTakenBeforeDying :type "Float (single-precision)") (HitLocation :type "Vector Structure"))
  (`KismetSystemLibrary.Delay` (`self.TimeBeforeDisolve`))
  (bind _returnvalue (`PrimitiveComponent.CreateDynamicMaterialInstance` (`self.SM_tentacles`) 0 (`PrimitiveComponent.GetMaterial` (`self.SM_tentacles`) 0) "None"))
  (bind (_direction _anim_curve) (`Timeline|Timeline_0` :!via `PlayFromStart`)
    (:`Update`
      (`MaterialInstanceDynamic.SetScalarParameterValue` _returnvalue "Amount" _anim_curve))
    (:`Finished`
      (`self.K2_DestroyActor`))))

(event `self.Health_Component_BP.OnDamage`
  (params (PointApplied :type "Float (single-precision)") (HitLocation :type "Vector Structure"))
  (`GameplayStatics.SpawnSoundAttached` "/Game/Sound/Sword_attack/HitCreature_Cue.HitCreature_Cue" (`self.SM_tentacles`) "None" (0.0 0.0 0.0) (struct) "KeepRelativeOffset" false 1.0 1.0 0.0 null null))

(fn `UserConstructionScript`)