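; BP_Levier is an interactable lever for the Catacombs level.
; Overlapping its sphere registers it as the player character's interaction and shows an "Activate" notification through the player controller; leaving clears both.
; Interact locks the lever, swings the stick with a timeline, fires the OnInteract dispatcher, then reverses after a short delay and unlocks once back at rest.
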(event `self.ReceiveBeginPlay`)

(event `self.Sphere.OnComponentBeginOverlap`
  (params (OverlappedComponent :type "PrimitiveComponent Object Reference") (OtherActor :type "Actor Object Reference") (OtherComp :type "PrimitiveComponent Object Reference") (OtherBodyIndex :type Integer) (bFromSweep :type Boolean) (SweepResult :type "HitResult Structure (by ref)"))
  (bind _asplayer_character_bp (cast `/Game/AdvancedLocomotionV4/Blueprints/CharacterLogic/PlayerCharacter_BP` OtherActor))
  (`/Game/AdvancedLocomotionV4/Blueprints/CharacterLogic/PlayerCharacter_BP.SetInteraction` _asplayer_character_bp self null null)
  (bind _asals_player_controller (cast `/Game/AdvancedLocomotionV4/Blueprints/CharacterLogic/ALS_Player_Controller` (`GameplayStatics.GetPlayerController` 0)))
  (`/Game/AdvancedLocomotionV4/Blueprints/CharacterLogic/ALS_Player_Controller.SendNotification` _asals_player_controller "Activate" 1000000000.0 self true))

(event `self.Sphere.OnComponentEndOverlap`
  (params (OverlappedComponent :type "PrimitiveComponent Object Reference") (OtherActor :type "Actor Object Reference") (OtherComp :type "PrimitiveComponent Object Reference") (OtherBodyIndex :type Integer))
  (bind _asplayer_character_bp (cast `/Game/AdvancedLocomotionV4/Blueprints/CharacterLogic/PlayerCharacter_BP` OtherActor))
  (`/Game/AdvancedLocomotionV4/Blueprints/CharacterLogic/PlayerCharacter_BP.ClearInteraction` _asplayer_character_bp self null null)
  (bind _asals_player_controller (cast `/Game/AdvancedLocomotionV4/Blueprints/CharacterLogic/ALS_Player_Controller` (`GameplayStatics.GetPlayerController` 0)))
  (`/Game/AdvancedLocomotionV4/Blueprints/CharacterLogic/ALS_Player_Controller.SendNotification` _asals_player_controller "" 0.0 self false))

(event `Interact`
  (if (not (`self.Locked`))
    (set `self.Locked` true)
    (bind (_direction _rotation) (`Timeline|LevierRotation` :!via `PlayFromStart` :!label _label)
      (:`Update`
        (`SceneComponent.K2_SetRelativeRotation` (`self.SM_Levier_Baton`) (`KismetMathLibrary.MakeRotator` (* _rotation 90.0)) false false))
      (:`Finished`
        (if (`|EnumEquality` _direction "Forward")
          (`self.OnInteract` self)
          (`KismetSystemLibrary.Delay` 3.0)
          (goto _label :!via `ReverseFromEnd`)
          (else
            (set `self.Locked` false)))))))

(fn `UserConstructionScript`)