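; Catacombs corridor Blueprint that procedurally dresses its static mesh with randomly chosen props in the construction script.
; Each slot randomly gets either one large prop or a random subset of small ones, placed at mesh sockets.
; A seeded stream picks mesh, offset, scale and optional yaw, but slot choices use unseeded RandomBool, so layouts are not fully seed-reproducible.
; Randomize rolls a new seed.
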(fn `AddMeshFromSlot`
  (params (Slot :type "/Game/Blueprints/LD/Catacombs/Slot_Struct Structure (by ref)"))
  (locals (Scale :type "Vector Structure") (Rotation :type "Rotator Structure" :default (struct)))
  (bind _staticmesh (`self.StaticMesh`))
  (bind _returnvalue (`KismetMathLibrary.RandomFloatInRangeFromStream` (.x (`.ScaleMin_4_239D26034F82534DD1C2ED9F174457C1` (break `/Game/Blueprints/LD/Catacombs/Slot_Struct` Slot))) (.x (`.ScaleMax_5_E5DEDD6847D0C8412CC2A59F2C065651` (break `/Game/Blueprints/LD/Catacombs/Slot_Struct` Slot))) (`self.Stream`)))
  (if `Slot_UniformScale?_8_C94FFD8E4079841152E3D39BD2D36F0D`
    (set `local.Scale` (`KismetMathLibrary.MakeVector` _returnvalue _returnvalue _returnvalue))
    (else
      (set `local.Scale` (`KismetMathLibrary.MakeVector` (`KismetMathLibrary.RandomFloatInRangeFromStream` (.x (`.ScaleMin_4_239D26034F82534DD1C2ED9F174457C1` (break `/Game/Blueprints/LD/Catacombs/Slot_Struct` Slot))) (.x (`.ScaleMax_5_E5DEDD6847D0C8412CC2A59F2C065651` (break `/Game/Blueprints/LD/Catacombs/Slot_Struct` Slot))) (`self.Stream`)) (`KismetMathLibrary.RandomFloatInRangeFromStream` (.y (`.ScaleMin_4_239D26034F82534DD1C2ED9F174457C1` (break `/Game/Blueprints/LD/Catacombs/Slot_Struct` Slot))) (.y (`.ScaleMax_5_E5DEDD6847D0C8412CC2A59F2C065651` (break `/Game/Blueprints/LD/Catacombs/Slot_Struct` Slot))) (`self.Stream`)) (`KismetMathLibrary.RandomFloatInRangeFromStream` (.z (`.ScaleMin_4_239D26034F82534DD1C2ED9F174457C1` (break `/Game/Blueprints/LD/Catacombs/Slot_Struct` Slot))) (.z (`.ScaleMax_5_E5DEDD6847D0C8412CC2A59F2C065651` (break `/Game/Blueprints/LD/Catacombs/Slot_Struct` Slot))) (`self.Stream`))))))
  (if `Slot_RandomRotation?_14_B0E9D43140BB2DBB50C0EBA8403B54D5`
    (set `local.Rotation` (`KismetMathLibrary.MakeRotator` 0.0 0.0 (`KismetMathLibrary.RandomFloatInRangeFromStream` 0.0 360.0 (`self.Stream`))))
    (else
      (set `local.Rotation` (`SceneComponent.GetSocketRotation` _staticmesh Slot_SocketName_20_75349F0B49704EA77C20A58048E27E18))))
  (bind _returnvalue_2 (`AddComponent|NODE_AddStaticMeshComponent-2` :`bManualAttachment` true :`RelativeTransform` (`KismetMathLibrary.MakeTransform` (+ (`SceneComponent.GetSocketLocation` _staticmesh Slot_SocketName_20_75349F0B49704EA77C20A58048E27E18) (`KismetMathLibrary.MakeVector` (`KismetMathLibrary.RandomFloatInRangeFromStream` 0.0 (.x (`.MaxOffset_11_854BE30449A67689FC41E4848FF87EA6` (break `/Game/Blueprints/LD/Catacombs/Slot_Struct` Slot))) (`self.Stream`)) (`KismetMathLibrary.RandomFloatInRangeFromStream` 0.0 (.y (`.MaxOffset_11_854BE30449A67689FC41E4848FF87EA6` (break `/Game/Blueprints/LD/Catacombs/Slot_Struct` Slot))) (`self.Stream`)) (`KismetMathLibrary.RandomFloatInRangeFromStream` 0.0 (.z (`.MaxOffset_11_854BE30449A67689FC41E4848FF87EA6` (break `/Game/Blueprints/LD/Catacombs/Slot_Struct` Slot))) (`self.Stream`)))) (`local.Rotation`) (`local.Scale`))))
  (`StaticMeshComponent.SetStaticMesh` _returnvalue_2 (`KismetArrayLibrary.Array_RandomFromStream` Slot_Mesh_21_238CFB3F4CB495AE12EBF591BD0A919B (`self.Stream`)))
  (`SceneComponent.K2_AttachToComponent` _returnvalue_2 (`self.StaticMesh`) "None" "KeepWorld" "KeepWorld" "KeepWorld" true))

(fn `Randomize`
  (set `self.Seed` (`KismetMathLibrary.RandomInteger` 9999999)))

(fn `UserConstructionScript`
  (`KismetMathLibrary.SetRandomStreamSeed` (`self.Stream`) (`self.Seed`))
  (for _array_element (`self.Slots`)
    (if (`KismetMathLibrary.RandomBool`)
      (bind (_largeslot _smallslots) (break `/Game/Blueprints/LD/Catacombs/SlotsContainer_Struct` _array_element))
      (`self.AddMeshFromSlot` _largeslot)
      (else
        (for _array_element_2 _smallslots
          (if (`KismetMathLibrary.RandomBool`)
            (`self.AddMeshFromSlot` _array_element_2)))))))