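; Catacombs puzzle actor with three concentric stone rings that levers rotate until their yaws line up.
; Each lever's Config entry lists ring moves in subdivision steps, animated on Tick over RotationDuration, ignoring new interactions meanwhile.
; The construction script scrambles the rings by applying each entry's moves in reverse NumberInitialUse times.
; Once CheckSolved finds alignment within half a step, it fires OnPuzzleSolved, plays a chime and animates a material Radius.
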(event `self.ReceiveBeginPlay`
  (for _array_element (`self.Config`)
    (add `/Game/Blueprints/LD/Catacombs/BP_Levier.OnInteract` (break `/Game/Blueprints/LD/PuzzleLeverConfig_Struct` _array_element) (delegate `OnInteractLevier`))))

(event `OnInteractLevier`
  (params (Levier :type "/Game/Blueprints/LD/Catacombs/BP_Levier Object Reference"))
  (if (and (== (`self.CurrentConfigRunning`) -1) (not (`self.CheckSolved`)))
    (for (_array_element _array_index) (`self.Config`)
      (if (== Levier (break `/Game/Blueprints/LD/PuzzleLeverConfig_Struct` _array_element))
        (set `self.CurrentConfigRunning` _array_index)
        (for _ (`.RingsMovements_10_D743BFFF4B9786E2C3302F9CC0BC4F65` (break `/Game/Blueprints/LD/PuzzleLeverConfig_Struct` _array_element))
          (`GameplayStatics.PlaySoundAtLocation` "/Game/Sound/StoneSlide_Cue.StoneSlide_Cue" (`SceneComponent.K2_GetComponentLocation` (`self.DefaultSceneRoot`)) (struct) 1.0 1.0 0.0 null null null))))))

(event `self.ReceiveTick`
  (params (DeltaSeconds :type "Float (single-precision)"))
  (bind _rotationduration (`self.RotationDuration`))
  (bind _sm_puzzle_cercle01 (`self.SM_Puzzle_Cercle01`))
  (bind _sm_puzzle_cercle01_2 (`self.SM_Puzzle_Cercle01`))
  (bind _sm_puzzle_cercle02 (`self.SM_Puzzle_Cercle02`))
  (bind _sm_puzzle_cercle03 (`self.SM_Puzzle_Cercle03`))
  (bind (_output_levier _output_ringsmovements) (break `/Game/Blueprints/LD/PuzzleLeverConfig_Struct` (`|GetArrayItem` (`self.Config`) (`self.CurrentConfigRunning`))))
  (if (!= (`self.CurrentConfigRunning`) -1)
    (set `self.Delta Seconds` DeltaSeconds)
    (bind _output_get (set `self.TimeElapsed` (+ (`self.TimeElapsed`) DeltaSeconds)))
    (if (> _output_get _rotationduration)
      (set `self.Delta Seconds` (- (`self.Delta Seconds`) (- _output_get _rotationduration))))
    (for _array_element _output_ringsmovements
      (switch `int` (break `/Game/Blueprints/LD/PuzzleRingConfig_Struct` _array_element)
        (:`1`
          (if (`.RotateOnLeft?_8_450A7EA24EA1C2777D9010BB15B0616D` (break `/Game/Blueprints/LD/PuzzleRingConfig_Struct` _array_element))
            (bind _returnvalue (* (/ (* (`.NumberOfRotation_9_71A47BE2465F82AA5711469195A87E71` (break `/Game/Blueprints/LD/PuzzleRingConfig_Struct` _array_element)) (/ 360.0 (`KismetMathLibrary.Conv_IntToDouble` (`self.NumberOfSubdiv`)))) (`self.RotationDuration`)) (`self.Delta Seconds`)))
            (`SceneComponent.K2_AddLocalRotation` _sm_puzzle_cercle01_2 (`KismetMathLibrary.MakeRotator` 0.0 0.0 _returnvalue) false false)
            (else
              (bind _returnvalue_2 (* _returnvalue -1.0))
              (`SceneComponent.K2_AddLocalRotation` _sm_puzzle_cercle01_2 (`KismetMathLibrary.MakeRotator` 0.0 0.0 _returnvalue_2) false false))))
        (:`2`
          (if (`.RotateOnLeft?_8_450A7EA24EA1C2777D9010BB15B0616D` (break `/Game/Blueprints/LD/PuzzleRingConfig_Struct` _array_element))
            (`SceneComponent.K2_AddLocalRotation` _sm_puzzle_cercle02 (`KismetMathLibrary.MakeRotator` 0.0 0.0 _returnvalue) false false)
            (else
              (`SceneComponent.K2_AddLocalRotation` _sm_puzzle_cercle02 (`KismetMathLibrary.MakeRotator` 0.0 0.0 _returnvalue_2) false false))))
        (:`3`
          (if (`.RotateOnLeft?_8_450A7EA24EA1C2777D9010BB15B0616D` (break `/Game/Blueprints/LD/PuzzleRingConfig_Struct` _array_element))
            (`SceneComponent.K2_AddLocalRotation` _sm_puzzle_cercle03 (`KismetMathLibrary.MakeRotator` 0.0 0.0 _returnvalue) false false)
            (else
              (`SceneComponent.K2_AddLocalRotation` _sm_puzzle_cercle03 (`KismetMathLibrary.MakeRotator` 0.0 0.0 _returnvalue_2) false false))))))
    (if (>= (`self.TimeElapsed`) (`self.RotationDuration`))
      (set `self.TimeElapsed` 0.0)
      (set `self.CurrentConfigRunning` -1)
      (if (`self.CheckSolved`)
        (`self.OnPuzzleSolved`)
        (`GameplayStatics.PlaySoundAtLocation` "/Game/Sound/86078__harpoyume__shine02.86078__harpoyume__shine02" (0.0 0.0 0.0) (struct) 1.0 1.0 0.0 null null null)
        (bind _returnvalue_3 (`PrimitiveComponent.CreateDynamicMaterialInstance` _sm_puzzle_cercle01 0 (`PrimitiveComponent.GetMaterial` _sm_puzzle_cercle01 0) "None"))
        (`PrimitiveComponent.SetMaterial` (`self.SM_Puzzle_Cercle02`) 0 _returnvalue_3)
        (`PrimitiveComponent.SetMaterial` (`self.SM_Puzzle_Cercle03`) 0 _returnvalue_3)
        (bind (_direction _radius) (`Timeline|SwitchOnDuration` :!via `PlayFromStart`)
          (:`Update`
            (`MaterialInstanceDynamic.SetScalarParameterValue` _returnvalue_3 "Radius" _radius)))))))

(fn `CheckSolved`
  (returns (IsSolved :type Boolean))
  (bind (_relativerotation_roll _relativerotation_pitch _relativerotation_yaw) (`KismetMathLibrary.BreakRotator` (`SceneComponent.RelativeRotation` (`self.SM_Puzzle_Cercle01`))))
  (bind (_relativerotation_roll_2 _relativerotation_pitch_2 _relativerotation_yaw_2) (`KismetMathLibrary.BreakRotator` (`SceneComponent.RelativeRotation` (`self.SM_Puzzle_Cercle02`))))
  (bind (_relativerotation_roll_3 _relativerotation_pitch_3 _relativerotation_yaw_3) (`KismetMathLibrary.BreakRotator` (`SceneComponent.RelativeRotation` (`self.SM_Puzzle_Cercle03`))))
  (bind _returnvalue (/ 180.0 (`KismetMathLibrary.Conv_IntToDouble` (`self.NumberOfSubdiv`))))
  (return (and (`KismetMathLibrary.NearlyEqual_FloatFloat` _relativerotation_yaw_2 _relativerotation_yaw_3 _returnvalue) (`KismetMathLibrary.NearlyEqual_FloatFloat` _relativerotation_yaw_3 _relativerotation_yaw _returnvalue))))

(fn `UserConstructionScript`
  (bind _sm_puzzle_cercle01 (`self.SM_Puzzle_Cercle01`))
  (bind _sm_puzzle_cercle02 (`self.SM_Puzzle_Cercle02`))
  (bind _sm_puzzle_cercle03 (`self.SM_Puzzle_Cercle03`))
  (for _array_element (`self.Config`)
    (for _array_element_2 (`.RingsMovements_10_D743BFFF4B9786E2C3302F9CC0BC4F65` (break `/Game/Blueprints/LD/PuzzleLeverConfig_Struct` _array_element))
      (switch `int` (break `/Game/Blueprints/LD/PuzzleRingConfig_Struct` _array_element_2)
        (:`1`
          (if (`.RotateOnLeft?_8_450A7EA24EA1C2777D9010BB15B0616D` (break `/Game/Blueprints/LD/PuzzleRingConfig_Struct` _array_element_2))
            (bind _returnvalue (* (* (`.NumberInitialUse_13_B8EB97CE4308BA9783237E894C392361` (break `/Game/Blueprints/LD/PuzzleLeverConfig_Struct` _array_element)) -1) (* (`.NumberOfRotation_9_71A47BE2465F82AA5711469195A87E71` (break `/Game/Blueprints/LD/PuzzleRingConfig_Struct` _array_element_2)) (/ 360.0 (`KismetMathLibrary.Conv_IntToDouble` (`self.NumberOfSubdiv`))))))
            (`SceneComponent.K2_AddLocalRotation` _sm_puzzle_cercle01 (`KismetMathLibrary.MakeRotator` 0.0 0.0 _returnvalue) false false)
            (else
              (bind _returnvalue_2 (* _returnvalue -1.0))
              (`SceneComponent.K2_AddLocalRotation` _sm_puzzle_cercle01 (`KismetMathLibrary.MakeRotator` 0.0 0.0 _returnvalue_2) false false))))
        (:`2`
          (if (`.RotateOnLeft?_8_450A7EA24EA1C2777D9010BB15B0616D` (break `/Game/Blueprints/LD/PuzzleRingConfig_Struct` _array_element_2))
            (`SceneComponent.K2_AddLocalRotation` _sm_puzzle_cercle02 (`KismetMathLibrary.MakeRotator` 0.0 0.0 _returnvalue) false false)
            (else
              (`SceneComponent.K2_AddLocalRotation` _sm_puzzle_cercle02 (`KismetMathLibrary.MakeRotator` 0.0 0.0 _returnvalue_2) false false))))
        (:`3`
          (if (`.RotateOnLeft?_8_450A7EA24EA1C2777D9010BB15B0616D` (break `/Game/Blueprints/LD/PuzzleRingConfig_Struct` _array_element_2))
            (`SceneComponent.K2_AddLocalRotation` _sm_puzzle_cercle03 (`KismetMathLibrary.MakeRotator` 0.0 0.0 _returnvalue) false false)
            (else
              (`SceneComponent.K2_AddLocalRotation` _sm_puzzle_cercle03 (`KismetMathLibrary.MakeRotator` 0.0 0.0 _returnvalue_2) false false))))))))