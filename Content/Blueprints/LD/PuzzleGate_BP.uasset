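; PuzzleGate_BP is a gate that opens when its referenced Puzzle02 puzzle is solved.
; BeginPlay binds to the puzzle's OnPuzzleSolved event and caches the mesh's starting relative location.
; On solve, it plays metal rattle and gate slam sounds at the world origin, then runs the OpenGate timeline.
; The timeline curve scales OpenOffset to slide the mesh from that start, without sweep.
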(event `self.ReceiveBeginPlay`
  (add `/Game/Blueprints/LD/Catacombs/BP_Puzzle.OnPuzzleSolved` (`self.Puzzle02`) (delegate `OnSolved`))
  (set `self.Relative Location` (`SceneComponent.RelativeLocation` (`self.StaticMeshComponent0`))))

(event `OnSolved`
  (`GameplayStatics.PlaySoundAtLocation` "/Game/Sound/160047__jorickhoofd__metal-rattle.160047__jorickhoofd__metal-rattle" (0.0 0.0 0.0) (struct) 1.0 1.0 0.0 null null null)
  (`GameplayStatics.PlaySoundAtLocation` "/Game/Sound/530061__magnuswaker__gates-of-hell-2-gate-slam-2.530061__magnuswaker__gates-of-hell-2-gate-slam-2" (0.0 0.0 0.0) (struct) 1.0 1.0 0.0 null null null)
  (bind (_direction _opencurve) (`Timeline|OpenGate`)
    (:`Update`
      (`SceneComponent.K2_SetRelativeLocation` (`self.StaticMeshComponent0`) (+ (`self.Relative Location`) (* (`self.OpenOffset`) _opencurve)) false false))))

(fn `UserConstructionScript`)