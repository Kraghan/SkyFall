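; Pillar lamp that fades its fire light in when the player comes near and out when they leave, unless flagged AlwaysOn.
; BeginPlay caches the intensity of the FireLight_BP child actor's light and sets the initial fade direction from the player's overlap with the sphere.
; Sphere overlap events play or reverse the SwitchLight timeline, whose LightFade track scales that cached intensity.
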(event `self.ReceiveBeginPlay`
  (bind _asfire_light_bp (cast `/Game/Blueprints/LD/Component/FireLight_BP` (`ChildActorComponent.ChildActor` (`self.FireLight_BP`))))
  (set `self.Intensity` (`LightComponentBase.Intensity` (`Light.LightComponent` _asfire_light_bp)))
  (if (`self.AlwaysOn`)
    _
    (elif (`PrimitiveComponent.IsOverlappingActor` (`self.Sphere`) (`GameplayStatics.GetPlayerCharacter` 0))
      (bind (_direction _lightfade) (`Timeline|SwitchLight` :!label _label)
        (:`Update`
          (bind _asfire_light_bp_2 (cast `/Game/Blueprints/LD/Component/FireLight_BP` (`ChildActorComponent.ChildActor` (`self.FireLight_BP`))))
          (`LightComponent.SetIntensity` (`Light.LightComponent` _asfire_light_bp_2) (* _lightfade (`self.Intensity`)))))
      (else
        (goto _label :!via `Reverse`)))))

(event `self.Sphere.OnComponentBeginOverlap`
  (params (OverlappedComponent :type "PrimitiveComponent Object Reference") (OtherActor :type "Actor Object Reference") (OtherComp :type "PrimitiveComponent Object Reference") (OtherBodyIndex :type Integer) (bFromSweep :type Boolean) (SweepResult :type "HitResult Structure (by ref)"))
  (if (and (== OtherActor (`GameplayStatics.GetPlayerCharacter` 0)) (not (`self.AlwaysOn`)))
    (goto _label)))

(event `self.Sphere.OnComponentEndOverlap`
  (params (OverlappedComponent :type "PrimitiveComponent Object Reference") (OtherActor :type "Actor Object Reference") (OtherComp :type "PrimitiveComponent Object Reference") (OtherBodyIndex :type Integer))
  (if (and (== (`GameplayStatics.GetPlayerCharacter` 0) OtherActor) (not (`self.AlwaysOn`)))
    (goto _label :!via `Reverse`)))

(fn `UserConstructionScript`)