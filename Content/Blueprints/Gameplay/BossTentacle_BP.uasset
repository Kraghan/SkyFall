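; BossTentacle_BP is a boss tentacle actor whose damage collision can be switched on and off.
; Its ToggleDamageCollision event sets the Capsule1 collision profile to Pawn when enabled and to NoCollision when disabled.
; It has no other active logic of its own: BeginPlay, overlap and Tick are disabled stubs, and the construction script only calls its parent.
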(event `ToggleDamageCollision`
  (params (`Enable?` :type Boolean))
  (bind _capsule1 (`self.Capsule1`))
  (if `Enable?`
    (`PrimitiveComponent.SetCollisionProfileName` _capsule1 "Pawn" true)
    (else
      (`PrimitiveComponent.SetCollisionProfileName` _capsule1 "NoCollision" true))))

(fn `UserConstructionScript`
  (`parent.UserConstructionScript`))