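; Health component that tracks its owner's current health and handles damage, healing and death.
; It binds to the owner's point damage event, treating Heal_DamageType as healing and anything else as damage, marked with a debug sphere.
; Both paths go through UpdateHealth, which clamps to the valid range and rejects changes once dead.
; Dispatchers report damage, blocked non-positive damage, heals and death, passing hit location for all but heals.
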(event `self.ReceiveBeginPlay`
  (`self.InitializeHealth`)
  (add `Actor.OnTakePointDamage` (`self.GetOwner`) (delegate `OnTakePointDamage`)))

(event `OnTakeDamage`
  (params (DamagedActor :type "Actor Object Reference") (Damage :type "Float (double-precision)") (DamageType :type "DamageType Object Reference") (InstigatedBy :type "Controller Object Reference") (DamageCauser :type "Actor Object Reference"))
  (cast `/Game/Blueprints/Gameplay/DamageType/Heal_DamageType` (stale `OnTakePointDamage` DamageType) :!label _label
    (:`then`
      (`self.ApplyHeal` (stale `OnTakePointDamage` Damage)))
    (:`CastFailed`
      (`self.ApplyDamage` (stale `OnTakePointDamage` Damage) (stale `OnTakePointDamage` HitLocation))
      (`KismetSystemLibrary.DrawDebugSphere` (stale `OnTakePointDamage` HitLocation) 25.0 12 (struct :`R` 1.0 :`A` 1.0) 5.0))))

(event `OnTakePointDamage`
  (params (DamagedActor :type "Actor Object Reference") (Damage :type "Float (double-precision)") (InstigatedBy :type "Controller Object Reference") (HitLocation :type "Vector Structure") (FHitComponent :type "PrimitiveComponent Object Reference") (BoneName :type Name) (ShotFromDirection :type "Vector Structure") (DamageType :type "DamageType Object Reference") (DamageCauser :type "Actor Object Reference"))
  (goto _label))

(fn `ApplyDamage`
  (params (Damage :type "Float (double-precision)") (HitLocation :type "Vector Structure"))
  (if (<= Damage 0.0)
    (`self.OnDamageBlocked` HitLocation)
    (else
      (bind _result (`/Engine/EditorBlueprintResources/StandardMacros.NegateFloat` Damage)
        (:`  `
          (bind _pointapplied (`self.Update Health` _result HitLocation))
          (if (!= _pointapplied 0.0)
            (`self.OnDamage` _pointapplied HitLocation)))))))

(fn `ApplyHeal`
  (params (Heal :type "Float (double-precision)"))
  (bind _pointapplied (`self.Update Health` Heal))
  (if (!= _pointapplied 0.0)
    (`self.OnHeal` _pointapplied)))

(fn `InitializeHealth`
  (if (<= (`self.InitHealth`) 0.0)
    (set `self.CurrentHealth` (`self.MaxHealth`))
    (elif (>= (`self.InitHealth`) (`self.MaxHealth`))
      (set `self.CurrentHealth` (`self.MaxHealth`))
      (else
        (set `self.CurrentHealth` (`self.InitHealth`))))))

(fn `IsDamaged`
  (returns (`IsDamaged?` :type Boolean))
  (return (!= (`self.CurrentHealth`) (`self.MaxHealth`))))

(fn `IsDead`
  (returns (`Dead?` :type Boolean))
  (return (== (`self.CurrentHealth`) 0.0)))

(fn `Update Health`
  (params (HealthModificationAmount :type "Float (double-precision)") (HitLocation :type "Vector Structure"))
  (returns (PointApplied :type "Float (double-precision)"))
  (locals (HealthBeforeUpdate :type "Float (double-precision)" :default 0.0))
  (if (`self.IsDead`)
    (`KismetSystemLibrary.PrintString` "Can't update health of a dead actor" true true (struct :`R` 1.0 :`A` 1.0))
    (elif (== HealthModificationAmount 0.0)
      (`KismetSystemLibrary.PrintString` "Trying to apply 0 damage / heal" true true (struct :`R` 1.0 :`A` 1.0))
      (else
        (set `local.HealthBeforeUpdate` (`self.CurrentHealth`))
        (bind _output_get (set `self.CurrentHealth` (`KismetMathLibrary.FClamp` (+ (`self.CurrentHealth`) (`local.HealthModificationAmount`)) 0.0 (`self.MaxHealth`))))
        (if (`self.IsDead`)
          (bind _returnvalue (`KismetMathLibrary.Abs` (- _output_get (`local.HealthBeforeUpdate`))))
          (`self.OnDie` _returnvalue (`local.HitLocation`)))
        (return _returnvalue))))
  (return 0.0))