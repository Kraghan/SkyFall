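; Melee sword actor that deals point damage through a capsule hitbox for its parent ALS character.
; ActivateHitBox enables the capsule and clears the hit list, so each actor with a health component is damaged once per activation.
; TargetCanBeDamaged selects the character's ActualDamage, or -1 when the target is blocking without attacking or is not an ALS character.
; Debug draws the active capsule, while hit spheres always draw.
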(event `self.ReceiveBeginPlay`
  (`self.DeactivateHitBox`)
  (bind _asals_anim_man_character_bp (cast `/Game/AdvancedLocomotionV4/Blueprints/CharacterLogic/ALS_AnimMan_CharacterBP` (`self.GetParentActor`)))
  (set `self.Character` _asals_anim_man_character_bp))

(event `self.ReceiveTick`
  (params (DeltaSeconds :type "Float (single-precision)"))
  (bind _capsule (`self.Capsule`))
  (if (and (`self.Debug`) (`ActorComponent.IsActive` (`self.Capsule`)))
    (`KismetSystemLibrary.DrawDebugCapsule` (`SceneComponent.K2_GetComponentLocation` _capsule) (`CapsuleComponent.GetScaledCapsuleHalfHeight` _capsule) (`CapsuleComponent.GetScaledCapsuleRadius` _capsule) (`SceneComponent.K2_GetComponentRotation` _capsule) (struct :`R` 1.0 :`A` 1.0) 0.0 2.0)))

(event `self.Capsule.OnComponentBeginOverlap`
  (params (OverlappedComponent :type "PrimitiveComponent Object Reference") (OtherActor :type "Actor Object Reference") (OtherComp :type "PrimitiveComponent Object Reference") (OtherBodyIndex :type Integer) (bFromSweep :type Boolean) (SweepResult :type "HitResult Structure (by ref)"))
  (bind _returnvalue (`self.K2_GetActorLocation` OtherActor))
  (bind _returnvalue_2 (`self.K2_GetActorLocation` (`self.Character`)))
  (bind _returnvalue_3 (`KismetMathLibrary.Normal` (- _returnvalue _returnvalue_2)))
  (bind _returnvalue_4 (+ _returnvalue_2 (* _returnvalue_3 10.0)))
  (`/Engine/EditorBlueprintResources/StandardMacros.IsValid` (`self.GetComponentByClass` OtherActor "/Game/Blueprints/Gameplay/Health_Component_BP.Health_Component_BP_C")
    (:`Is Valid`
      (if (and (not (`BlueprintSetLibrary.Set_Contains` (`self.DamagedActor`) OtherActor)) (!= (`self.Character`) OtherActor) (`ActorComponent.IsActive` (`self.Capsule`)))
        (if (`self.TargetCanBeDamaged` OtherActor)
          (set `self.Damage` (`/Game/AdvancedLocomotionV4/Blueprints/CharacterLogic/ALS_AnimMan_CharacterBP.ActualDamage` (`self.Character`)))
          (else
            (set `self.Damage` -1.0)))
        (`GameplayStatics.ApplyPointDamage` OtherActor (`self.Damage`) _returnvalue_3 (`GameplayStatics.MakeHitResult` false false 0.0 0.0 _returnvalue_4 _returnvalue_4 (0.0 0.0 1.0) (0.0 0.0 1.0) null OtherActor OtherComp) (`Pawn.GetController` (`self.Character`)) self "/Script/Engine.DamageType")
        (`BlueprintSetLibrary.Set_Add` (`self.DamagedActor`) OtherActor)
        (`KismetSystemLibrary.DrawDebugSphere` (`self.K2_GetActorLocation` (`self.Character`)) 20.0 12 (struct :`B` 1.0 :`A` 1.0) 5.0 2.0)
        (`KismetSystemLibrary.DrawDebugSphere` _returnvalue 20.0 12 (struct :`G` 1.0 :`A` 1.0) 5.0 2.0)))))

(event `ActivateHitBox`
  (`ActorComponent.Activate` (`self.Capsule`) true)
  (`BlueprintSetLibrary.Set_Clear` (`self.DamagedActor`)))

(event `DeactivateHitBox`
  (`ActorComponent.Deactivate` (`self.Capsule`)))

(fn `TargetCanBeDamaged`
  (params (Actor :type "Actor Object Reference"))
  (returns (ReturnValue :type Boolean))
  (bind _asals_anim_man_character_bp (cast `/Game/AdvancedLocomotionV4/Blueprints/CharacterLogic/ALS_AnimMan_CharacterBP` Actor))
  (if (`/Game/AdvancedLocomotionV4/Blueprints/CharacterLogic/ALS_AnimMan_CharacterBP.IsAttacking?` _asals_anim_man_character_bp)
    (return true)
    (else
      (return (not (`/Game/AdvancedLocomotionV4/Blueprints/CharacterLogic/ALS_AnimMan_CharacterBP.IsBlocking?` _asals_anim_man_character_bp))))))

(fn `UserConstructionScript`)