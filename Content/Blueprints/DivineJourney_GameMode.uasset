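; DivineJourney_GameMode is a game mode that spawns the player at the last recorded checkpoint.
; Its ChoosePlayerStart override reads LastCheckPointTag from SkyfallGameInstance_BP and returns the first Checkpoint_BP actor with a matching CheckpointTag.
; With no match it falls back to the parent's choice, but a failed game instance cast stops before that fallback.
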(fn `ChoosePlayerStart`
  (params (Player :type "Controller Object Reference"))
  (returns (ReturnValue :type "Actor Object Reference"))
  (bind _asskyfall_game_instance_bp (cast `/Game/Blueprints/SkyfallGameInstance_BP` (`GameplayStatics.GetGameInstance`)))
  (bind _outactors (`GameplayStatics.GetAllActorsOfClass` "/Game/Blueprints/Checkpoint_BP.Checkpoint_BP_C"))
  (for _array_element _outactors
    (if (== (`/Game/Blueprints/Checkpoint_BP.CheckpointTag` _array_element) (`/Game/Blueprints/SkyfallGameInstance_BP.LastCheckPointTag` _asskyfall_game_instance_bp))
      (return _array_element)))
  (bind _returnvalue (`parent.ChoosePlayerStart` Player))
  (return _returnvalue))

(fn `UserConstructionScript`)