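; AI controller for BP_Boss that runs the Boss_BT behavior tree.
; On possess it caches the boss, starts the tree and seeds the Blackboard with the player character as Target, Spawning on and Attacking off.
; Each tick it copies the boss's IsInSpawn flag into the Spawning key while the boss is valid.
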(event `self.ReceivePossess`
  (params (PossessedPawn :type "Pawn Object Reference"))
  (bind _asbp_boss (cast `/Game/Blueprints/Character/BP_Boss` PossessedPawn))
  (set `self.As BP Boss` _asbp_boss)
  (`self.RunBehaviorTree` "/Game/Blueprints/AI/Boss_BT.Boss_BT")
  (`BlackboardComponent.SetValueAsObject` (`self.Blackboard`) (`self.Target`) (`GameplayStatics.GetPlayerCharacter` 0))
  (`BlackboardComponent.SetValueAsBool` (`self.Blackboard`) (`self.Spawning`) true)
  (`BlackboardComponent.SetValueAsBool` (`self.Blackboard`) (`self.Attacking`) false))

(event `self.ReceiveTick`
  (params (DeltaSeconds :type "Float (single-precision)"))
  (bind _as_bp_boss (`self.As BP Boss`)
    (:`then`
      (`BlackboardComponent.SetValueAsBool` (`self.Blackboard`) (`self.Spawning`) (`/Game/Blueprints/Character/BP_Boss.IsInSpawn` _as_bp_boss)))
    (:`else`)))

(fn `UserConstructionScript`)